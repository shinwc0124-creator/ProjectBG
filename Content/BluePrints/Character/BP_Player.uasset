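; Player character Blueprint with movement, look, free look and item pickup.
; Free look disables controller yaw and moves relative to the saved rotation; on release a timeline lerps control rotation back, then restores yaw.
; Pickup reads a DT_ItemInfo row, adds HP, Attack and Speed, sets the weapon and updates the HUD widget.
; It also stores a pose state; EventGraph holds only unwired, annotated data-table reference nodes.
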(event Custom|OnFreeLookEnded
  (Timeline|Timeline PlayFromStart
    (:Update
      (Pawn|SetControlRotation (Pawn|GetController) (Math|Rotator|Lerp(Rotator) (Variables|FreeLook|GetEnd%20Rotation) (Variables|FreeLook|GetStart%20Rotation) 0.0 true)))
    (:Finished
      (Variables|Default|SetbUseControllerRotationYaw true))))

(fn ConstructionScript)

(fn InputTurn
  (params (X%20Axis :type Float%20%28double-precision%29))
  (Pawn|Input|AddControllerYawInput X%20Axis))

(fn InputLookUp
  (params (Y%20Axis :type Float%20%28double-precision%29))
  (Pawn|Input|AddControllerPitchInput Y%20Axis))

(fn Move
  (params (bIs%20Forward :type Boolean) (Axis%20Value :type Float%20%28double-precision%29))
  (bind _result (CallFunction|GetMoveRotation))
  (if bIs%20Forward
    (Pawn|Input|AddMovementInput (Math|Vector|GetForwardVector _result) Axis%20Value false)
    (else
      (Pawn|Input|AddMovementInput (Math|Vector|GetRightVector _result) Axis%20Value false))))

(fn FreeLook
  (params (bIs%20Pressed :type Boolean))
  (bind _returnvalue (Pawn|GetControlRotation :!class /Script/Engine.Pawn))
  (if bIs%20Pressed
    (Variables|FreeLook|SetStart%20Rotation _returnvalue)
    (Variables|Default|SetbUseControllerRotationYaw false)
    (else
      (Variables|FreeLook|SetEnd%20Rotation _returnvalue)
      (CallFunction|OnFreeLookEnded))))

(fn GetMoveRotation
  (return (Math|Rotator|SelectRotator (CallFunction|GetYawOnlyRotation self) (Variables|FreeLook|GetStart%20Rotation) (Variables|Default|GetbUseControllerRotationYaw))))

(fn UpdatePoseState
  (params (New%20State :type E_PoseState%20Enum :default "NewEnumerator0"))
  (Variables|Default|SetCurrentPoseState New%20State))

(fn OnPickUp
  (params (Row%20Name :type Name))
  (bind _returnvalue (Utilities|GetDataTableRow "/Game/BluePrints/Character/Test/DT_ItemInfo.DT_ItemInfo" Row%20Name)
    (:then
      (LocalVariables|SetItemInfo _returnvalue)
      (Utilities|FlowControl|Sequence
        (:then_0
          (Variables|Default|SetHP (+ (.hp (LocalVariables|GetItemInfo)) (Variables|Default|GetHP)))
          (Variables|Default|SetAttack (+ (.attack (LocalVariables|GetItemInfo)) (Variables|Default|GetAttack)))
          (Variables|Default|SetSpeed (+ (.speed (LocalVariables|GetItemInfo)) (Variables|Default|GetSpeed)))
          (Variables|Default|SetWeapon (.weapon (LocalVariables|GetItemInfo))))
        (:then_1
          (bind _asbp_hud (Utilities|Casting|CastToBP_HUD (HUD|GetHUD (Game|GetPlayerController 0))))
          (Default|UpdateImage (Variables|/Game/BluePrints/Character/BP_HUD.BP_HUD_C|GetTestWidget _asbp_hud) (.itemimage (LocalVariables|GetItemInfo)))
          (Default|UpdateText (Variables|/Game/BluePrints/Character/BP_HUD.BP_HUD_C|GetTestWidget _asbp_hud) (Utilities|Text|ToText(Integer) (Variables|Default|GetHP)) (Utilities|Text|ToText(Integer) (Variables|Default|GetAttack)) (Utilities|Text|ToText(Integer) (Variables|Default|GetSpeed)) (.weapon (LocalVariables|GetItemInfo))))))))