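; Player controller that routes movement, look, free look, jump, walk/run and crouch/prone input to BP_Player.
; Pose changes resolve target pose and transition time from data tables, pausing movement on a timer for timed transitions.
; Per-pose table rows also drive control pitch limits and spring arm height, both blended with timelines.
; Tick prints move state and speed for debugging.
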(event Custom|SetEnabledMove
  ;[0.15 0.15 0.15 0.5] 포즈변경
  (Variables|Move|SetbIs%20EnableMove true))

(event Custom|OnMovementStateChanged
  (params (bIsMoving :type Boolean))
  (Camera|UpdateCameraHeigth bIsMoving))

(event EventTick
  (params (DeltaSeconds :type Float%20%28single-precision%29))
  (bind _player_ref (Variables|Ref|GetPlayer%20Ref))
  (Development|PrintText (Utilities|Text|FormatText "Pose : {pose} Speed : {speed}" (Utilities|String|EnumtoString (Variables|/Game/BluePrints/Character/BP_Player.BP_Player_C|GetCurrentMoveState _player_ref)) (Math|Vector|VectorLength (Transformation|GetVelocity _player_ref))) true true "(R=0.000000,G=0.660000,B=1.000000,A=1.000000)" 0.0))

(event EventBeginPlay
  ;[0.15 0.15 0.15 0.5] 참조캐싱
  (bind _asbp_player (Utilities|Casting|CastToBP_Player (Game|GetPlayerCharacter 0)))
  (Variables|Ref|SetPlayer%20Ref _asbp_player)
  ;[0.15 0.15 0.15 0.5] 카메라 각도 제한 초기화
  (Camera|UpdatePitchLimits "NewEnumerator0")
  (EventDispatchers|BindEventtoOnMovementStateChanged (Variables|Ref|GetPlayer%20Ref) (delegate Custom|OnMovementStateChanged))
  (Default|CachedWalkSpeedbyPose (Variables|Ref|GetPlayer%20Ref)))

(event Input|ActionEvents|InputActionFreeLook
  (params (Key :type Key%20Structure :default "None"))
  (bind _player_ref (Variables|Ref|GetPlayer%20Ref))
  ;[0.15 0.15 0.15 0.5] 자유시점
  (:Pressed
    (Default|FreeLook _player_ref true))
  (:Released
    (Default|FreeLook _player_ref false)))

(event Input|ActionEvents|InputActionWalk
  (params (Key :type Key%20Structure :default "None"))
  (bind _player_ref (Variables|Ref|GetPlayer%20Ref))
  ;[0.15 0.15 0.15 0.5] Walk : 누르면 상태가 Walk, 안누르면 Jog
  (:Pressed
    (Variables|/Game/BluePrints/Character/BP_Player.BP_Player_C|SetbIsWalkPressed _player_ref true)
    (Default|EvaluateMoveState _player_ref :!label _label)
    (Default|CachedWalkSpeedbyPose _player_ref))
  (:Released
    (Variables|/Game/BluePrints/Character/BP_Player.BP_Player_C|SetbIsWalkPressed _player_ref false)
    (goto _label)))

(event Input|ActionEvents|InputActionRun
  (params (Key :type Key%20Structure :default "None"))
  (bind _player_ref (Variables|Ref|GetPlayer%20Ref))
  ;[0.15 0.15 0.15 0.5] Run : 누르면 상태가 Run, 안누르면Jog
  (:Pressed
    (Variables|/Game/BluePrints/Character/BP_Player.BP_Player_C|SetbIsRunPressed _player_ref true)
    (Default|EvaluateMoveState _player_ref :!label _label)
    (Default|CachedWalkSpeedbyPose _player_ref))
  (:Released
    (Variables|/Game/BluePrints/Character/BP_Player.BP_Player_C|SetbIsRunPressed _player_ref false)
    (goto _label)))

(event Input|ActionEvents|InputActionCrouch
  (params (Key :type Key%20Structure :default "None"))
  (bind _player_ref (Variables|Ref|GetPlayer%20Ref))
  (bind _bis_weapon_equipped (Variables|/Game/BluePrints/Character/BP_Player.BP_Player_C|GetbIs%20Weapon%20Equipped _player_ref))
  (bind _currentposestate (Variables|/Game/BluePrints/Character/BP_Player.BP_Player_C|GetCurrentPoseState _player_ref))
  (bind (_transitiontime _topose) (Pose|OnTransitionTimer _bis_weapon_equipped "NewEnumerator1" _currentposestate))
  ;[0.15 0.15 0.15 0.5] 포즈변경
  (:Pressed
    (Pose|UpdatePose _transitiontime _topose)))

(event Input|ActionEvents|InputActionProne
  (params (Key :type Key%20Structure :default "None"))
  (bind _player_ref (Variables|Ref|GetPlayer%20Ref))
  (bind _currentposestate (Variables|/Game/BluePrints/Character/BP_Player.BP_Player_C|GetCurrentPoseState _player_ref))
  (bind _bis_weapon_equipped (Variables|/Game/BluePrints/Character/BP_Player.BP_Player_C|GetbIs%20Weapon%20Equipped _player_ref))
  (bind (_transitiontime _topose) (Pose|OnTransitionTimer _bis_weapon_equipped "NewEnumerator2" _currentposestate))
  ;[0.15 0.15 0.15 0.5] 포즈변경
  (:Pressed
    (Pose|UpdatePose _transitiontime _topose)))

(event Input|ActionEvents|InputActionJump
  (params (Key :type Key%20Structure :default "None"))
  (bind _player_ref (Variables|Ref|GetPlayer%20Ref))
  (bind _player_ref_2 (Variables|Ref|GetPlayer%20Ref))
  (bind _currentposestate (Variables|/Game/BluePrints/Character/BP_Player.BP_Player_C|GetCurrentPoseState _player_ref_2))
  (bind _bis_weapon_equipped (Variables|/Game/BluePrints/Character/BP_Player.BP_Player_C|GetbIs%20Weapon%20Equipped _player_ref))
  (bind (_transitiontime _topose) (Pose|OnTransitionTimer _bis_weapon_equipped "NewEnumerator0" _currentposestate))
  ;[0.15 0.15 0.15 0.5] 포즈변경
  (:Pressed
    (if (Utilities|Enum|Equal(Enum) _currentposestate "NewEnumerator0")
      (Character|Jump (Variables|Ref|GetPlayer%20Ref))
      (else
        (Pose|UpdatePose _transitiontime _topose)))))

(event Input|AxisEvents|InputAxisTurn
  (params (AxisValue :type Float%20%28single-precision%29))
  ;[0.15 0.15 0.15 0.5] 카메라 회전
  (Default|InputTurn (Variables|Ref|GetPlayer%20Ref) AxisValue))

(event Input|AxisEvents|InputAxisLookUp
  (params (AxisValue :type Float%20%28single-precision%29))
  ;[0.15 0.15 0.15 0.5] 카메라 회전
  (bind _returnvalue (Camera|LimitPitchAngle AxisValue))
  (if _returnvalue
    (Default|InputLookUp (Variables|Ref|GetPlayer%20Ref) AxisValue)))

(event Input|AxisEvents|InputAxisMoveForward
  (params (AxisValue :type Float%20%28single-precision%29))
  (bind _player_ref (Variables|Ref|GetPlayer%20Ref))
  ;[0.15 0.15 0.15 0.5] 캐릭터 이동
  (if (Variables|Move|GetbIs%20EnableMove)
    (Default|UpdateDirectionalSpeed _player_ref)
    (Default|Move _player_ref true AxisValue)))

(event Input|AxisEvents|InputAxisMoveRight
  (params (AxisValue :type Float%20%28single-precision%29))
  (bind _player_ref (Variables|Ref|GetPlayer%20Ref))
  ;[0.15 0.15 0.15 0.5] 캐릭터 이동
  (if (Variables|Move|GetbIs%20EnableMove)
    (Default|UpdateDirectionalSpeed _player_ref)
    (Default|Move _player_ref false AxisValue)))

(event Custom|ChangePitchLimit
  (params (CurrentRotator :type Rotator) (TargetRotator :type Rotator))
  (bind _alpha (Timeline|Timeline_0 PlayFromStart)
    (:Update
      (Pawn|SetControlRotation (Math|Rotator|Lerp(Rotator) CurrentRotator TargetRotator _alpha true)))))

(event Custom|SpringarmOffset
  (params (CurrentOffset :type Vector) (TargetOffset :type Vector))
  (bind _alpha (Timeline|Timeline PlayFromStart)
    (:Update
      (Variables|/Script/Engine.SpringArmComponent|SetSocketOffset (Variables|/Game/BluePrints/Character/BP_Player.BP_Player_C|GetSpringArm (Variables|Ref|GetPlayer%20Ref)) (Math|Vector|Lerp(Vector) CurrentOffset TargetOffset _alpha)))))

(fn ConstructionScript)

(fn TryGetPoseTransition
  (params (TargetPose :type E_PoseState%20Enum :default "NewEnumerator0") (FromPose :type E_PoseState%20Enum :default "NewEnumerator0"))
  (bind _returnvalue (Utilities|GetDataTableRow "/Game/BluePrints/Datas/DataTables/Character/DT_TransitionRule.DT_TransitionRule" (Utilities|String|StringToName (Utilities|String|Append (Utilities|String|EnumtoString TargetPose) "_" (Utilities|String|EnumtoString FromPose))))
    (:then
      (return (.topose _returnvalue)))))

(fn OnTransitionTimer
  (params (bIsWeaponWEquipped :type Boolean) (TargetPose :type E_PoseState%20Enum :default "NewEnumerator0") (FromPose :type E_PoseState%20Enum :default "NewEnumerator0"))
  (LocalVariables|SetReturnPose (Pose|TryGetPoseTransition TargetPose FromPose))
  (bind _returnvalue (Utilities|GetDataTableRow "/Game/BluePrints/Datas/DataTables/Character/DT_ProneTime.DT_ProneTime" (Utilities|String|StringToName (Utilities|String|Append (Utilities|String|ToString(Boolean) bIsWeaponWEquipped) "_" (Utilities|String|EnumtoString FromPose) "_" (Utilities|String|EnumtoString (LocalVariables|GetReturnPose)))))
    (:then
      _)
    (:RowNotFound
      _))
  (return (.sec _returnvalue) (LocalVariables|GetReturnPose)))

(fn UpdatePose
  (params (WaitTime :type Float%20%28double-precision%29) (ToPose :type E_PoseState%20Enum :default "NewEnumerator0"))
  (Utilities|FlowControl|Sequence
    (:then_0
      (if (!= WaitTime 0.0)
        (Variables|Move|SetbIs%20EnableMove false)
        (Utilities|Time|SetTimerbyEvent (EventDispatchers|CreateEvent :!event Custom|SetEnabledMove) WaitTime)
        (Default|UpdatePoseState (Variables|Ref|GetPlayer%20Ref) ToPose)
        (else
          (Default|UpdatePoseState (Variables|Ref|GetPlayer%20Ref) ToPose))))
    (:then_1
      (Camera|UpdatePitchLimits ToPose)
      (Camera|UpdateCameraHeigth (Variables|/Game/BluePrints/Character/BP_Player.BP_Player_C|GetbIs%20Weapon%20Equipped (Variables|Ref|GetPlayer%20Ref)))
      (Default|CachedWalkSpeedbyPose (Variables|Ref|GetPlayer%20Ref)))))

(fn UpdatePitchLimits
  (params (NewState :type E_PoseState%20Enum :default "NewEnumerator0"))
  (bind _returnvalue (Pawn|GetControlRotation :!class /Script/Engine.Controller))
  (Utilities|FlowControl|Sequence
    (:then_0
      (bind _returnvalue_2 (Utilities|GetDataTableRow "/Game/BluePrints/Datas/DataTables/Character/DT_PitchLimit.DT_PitchLimit" (Utilities|String|StringToName (Utilities|String|EnumtoString NewState)))
        (:then
          (Variables|Camera|SetCachedTopLimit (.toplimit _returnvalue_2))
          (Variables|Camera|SetCachedBotLimit (.bottomlimit _returnvalue_2)))))
    (:then_1
      (if (not (or (< (.pitch _returnvalue) (Variables|Camera|GetCachedBotLimit)) (> (.pitch _returnvalue) (Variables|Camera|GetCachedTopLimit))))
        (if (< (Math|Float|Absolute(Float) (- (.pitch _returnvalue) (Variables|Camera|GetCachedTopLimit))) (Math|Float|Absolute(Float) (- (.pitch _returnvalue) (Variables|Camera|GetCachedBotLimit))))
          (CallFunction|ChangePitchLimit (.CurrentRotator (Camera|MakeViewRotator (Variables|Camera|GetCachedTopLimit))) (.TargetRotator (Camera|MakeViewRotator (Variables|Camera|GetCachedTopLimit))))
          (else
            (CallFunction|ChangePitchLimit (.CurrentRotator (Camera|MakeViewRotator (Variables|Camera|GetCachedBotLimit))) (.TargetRotator (Camera|MakeViewRotator (Variables|Camera|GetCachedBotLimit))))))))))

(fn LimitPitchAngle
  (params (Axis :type Float%20%28double-precision%29))
  (bind _returnvalue (Class|PlayerController|GetDeprecatedInputPitchScale))
  (bind _returnvalue_2 (Pawn|GetControlRotation :!class /Script/Engine.Controller))
  (bind _returnvalue_3 (* _returnvalue Axis))
  (bind _returnvalue_4 (+ (.pitch _returnvalue_2) _returnvalue_3))
  (return (or (> _returnvalue_4 (Variables|Camera|GetCachedBotLimit)) (< _returnvalue_4 (Variables|Camera|GetCachedBotLimit)))))

(fn MakeViewRotator
  (params (LimitPitch :type Float%20%28double-precision%29))
  (bind _returnvalue (Pawn|GetControlRotation :!class /Script/Engine.Controller))
  (bind (_roll _pitch _yaw) (Math|Rotator|BreakRotator _returnvalue))
  (return _returnvalue (Math|Rotator|MakeRotator _roll LimitPitch _yaw)))

(fn UpdateCameraHeigth
  (params (bIsMovingNow :type Boolean))
  (bind _player_ref (Variables|Ref|GetPlayer%20Ref))
  (bind _player_ref_2 (Variables|Ref|GetPlayer%20Ref))
  (bind _currentposestate (Variables|/Game/BluePrints/Character/BP_Player.BP_Player_C|GetCurrentPoseState _player_ref_2))
  (bind _springarm (Variables|/Game/BluePrints/Character/BP_Player.BP_Player_C|GetSpringArm _player_ref))
  (bind _socketoffset (Variables|/Script/Engine.SpringArmComponent|GetSocketOffset _springarm))
  (Utilities|FlowControl|Sequence
    (:then_0
      (LocalVariables|SetCurrentPose (Utilities|String|EnumtoString _currentposestate))
      (if (Utilities|Enum|NotEqual(Enum) _currentposestate "NewEnumerator1")
        ;[0.15 0.15 0.15 0.5] Crouch가 아니라면 현재 상태가 곧 RowName
        (LocalVariables|SetRowName (LocalVariables|GetCurrentPose))
        (else
          (LocalVariables|SetRowName (LocalVariables|GetCurrentPose))
          (if (Variables|Move|GetbIs%20EnableMove)
            (LocalVariables|SetRowName (Utilities|String|Append (LocalVariables|GetRowName) "_" (Utilities|String|ToString(Boolean) (Variables|/Game/BluePrints/Character/BP_Player.BP_Player_C|GetbIs%20Weapon%20Equipped (Variables|Ref|GetPlayer%20Ref))) "_Move"))))))
    (:then_1
      (bind _returnvalue (Utilities|GetDataTableRow "/Game/BluePrints/Datas/DataTables/Character/DT_CameraHeight.DT_CameraHeight" (Utilities|String|StringToName (LocalVariables|GetRowName)))
        (:then
          (Variables|Default|SetTarget _returnvalue)
          (Variables|Default|SetTargetOffset (Math|Vector|MakeVector (.x _socketoffset) (.y _socketoffset) (.height (Variables|Default|GetTarget))))
          (CallFunction|SpringarmOffset (Variables|/Script/Engine.SpringArmComponent|GetSocketOffset _springarm) (Variables|Default|GetTargetOffset)))))))