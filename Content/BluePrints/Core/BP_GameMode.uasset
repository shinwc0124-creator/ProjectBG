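; Game mode that holds the logic for generating item groups in the level from data tables; BeginPlay is empty here.
; GenerateItem spawns a BP_ItemGroup at each DT_ItemGroupLocation row, then rolls an item count and adds that many random types to ItemTypeArray.
; Count and type are weighted picks: each table value is repeated Percent times in an array, then one is chosen at random.
; ItemTypeArray is not passed to the spawned groups here.
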(event EventBeginPlay)

(fn ConstructionScript)

(fn GenerateItem
  (bind _outrownames (DataTable|GetDataTableRowNames "/Game/BluePrints/Datas/DataTables/ItemGeneration/DT_ItemGroupLocation.DT_ItemGroupLocation"))
  (for _array_element _outrownames
    (bind _returnvalue (Utilities|GetDataTableRow "/Game/BluePrints/Datas/DataTables/ItemGeneration/DT_ItemGroupLocation.DT_ItemGroupLocation" _array_element)
      (:then
        (Game|SpawnActorfromClass "/Game/BluePrints/Items/BP_ItemGroup.BP_ItemGroup_C" (Math|Transform|MakeTransform (.location _returnvalue) "0, 0, 0" "1.000000,1.000000,1.000000") "Undefined" "MultiplyWithRoot" 0 0)
        (bind _number (CallFunction|RandomItemNumber))
        (for _index (range 1 _number)
          (bind _newparam (CallFunction|RandomItemType))
          (Utilities|Array|Add (LocalVariables|GetItemTypeArray) _newparam))))))

(fn RandomItemNumber
  (bind _outrownames (DataTable|GetDataTableRowNames "/Game/BluePrints/Datas/DataTables/ItemGeneration/DT_ItemProbability.DT_ItemProbability"))
  (for _array_element _outrownames
    (bind _returnvalue (Utilities|GetDataTableRow "/Game/BluePrints/Datas/DataTables/ItemGeneration/DT_ItemProbability.DT_ItemProbability" _array_element)
      (:then
        (for _index (range 1 (.percent _returnvalue))
          (Utilities|Array|Add (LocalVariables|GetNumberArray) (.number _returnvalue))))))
  (return (.OutItem (Utilities|Array|Random (LocalVariables|GetNumberArray)))))

(fn RandomItemType
  (bind _outrownames (DataTable|GetDataTableRowNames "/Game/BluePrints/Datas/DataTables/ItemGeneration/DT_ItemTypeProbabilty.DT_ItemTypeProbabilty"))
  (for _array_element _outrownames
    (bind _returnvalue (Utilities|GetDataTableRow "/Game/BluePrints/Datas/DataTables/ItemGeneration/DT_ItemTypeProbabilty.DT_ItemTypeProbabilty" _array_element)
      (:then
        (for _index (range 1 (.percent _returnvalue))
          (Utilities|Array|Add (LocalVariables|GetItemType) (.itemtype _returnvalue))))))
  (return (.OutItem (Utilities|Array|Random (LocalVariables|GetItemType)))))